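; BP_GameManager is a game manager Blueprint for a top-down game that handles startup and holds an early floor-generation routine.
; On BeginPlay it caches the player character, then creates Widget_Hud and adds it to the viewport.
; GenerateFloor1 picks a random room count between half and the full maximum, but only spawns BP_RoomStart.
; Nothing in this file calls that routine or uses the count.
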(event `self.ReceiveBeginPlay`
  ;[1 1 1] Initialize
  (bind _topdowncharacter (`/Game/Managers/BFL_GeneralFunctions.GetPlayer`))
  (set `self.Top Down Character` _topdowncharacter)
  (`self.CreateHUD`))

(fn `CreateHUD`
  (bind _returnvalue (`|CreateWidget` "/Game/UI/HUD/Widget_Hud.Widget_Hud_C"))
  (bind _output_get (set `self.Widget_HUD` _returnvalue))
  (`UserWidget.AddToViewport` _output_get 0)
  (return))

(fn `GenerateFloor_1`
  (locals (MaxNumberOfRoomsLocalvar :type Integer :default 0))
  (bind _maxnumberofrooms (`self.MaxNumberOfRooms`))
  (set `local.MaxNumberOfRoomsLocalvar` (`KismetMathLibrary.RandomIntegerInRange` (/ _maxnumberofrooms 2) _maxnumberofrooms))
  (`|SpawnActorFromClass` "/Game/Rooms/BP_RoomStart.BP_RoomStart_C" (`KismetMathLibrary.MakeTransform` (0.0 0.0 0.0)) "Undefined" "MultiplyWithRoot" null null))

(fn `UserConstructionScript`)